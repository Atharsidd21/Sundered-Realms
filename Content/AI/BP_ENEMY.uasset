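; Enemy character Blueprint, usable as a boss, that plays melee attack montages, takes damage and ragdolls on death.
; Damage lowers a BPCStats value tied to a healthbar widget and halts walking during the hit-react montage.
; Sword hits come from a looping-timer sphere trace with a short re-hit cooldown, using boss-specific endpoints when flagged.
; A point trace deals big-attack area damage with sound, shake and particles; a trigger overlap toggles the healthbar.
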(event `self.ReceiveBeginPlay`
  (bind _aswb_enemy_healthbar (cast `/Game/UI/WB_EnemyHealthbar` (`WidgetComponent.GetWidget` (`self.Widget`))))
  (`/Game/BluePrints/BPC_Stats.Set Health Progress BAR ` (`self.BPC_Stats`) (`/Game/UI/WB_EnemyHealthbar.healthbar` _aswb_enemy_healthbar))
  (`SkinnedMeshComponent.HideBoneByName` (`self.Enemy`) "weapon_r" "PBO_None")
  (set `self.Initial Walk Speed` (`CharacterMovementComponent.MaxWalkSpeed` (`self.CharacterMovement`))))

(event `self.ReceiveAnyDamage`
  (params (Damage :type "Float (single-precision)") (DamageType :type "DamageType Object Reference") (InstigatedBy :type "Controller Object Reference") (DamageCauser :type "Actor Object Reference"))
  (`/Game/BluePrints/BPC_Stats.increase value` (`self.BPC_Stats`) "NewEnumerator0" (* Damage -1.0))
  (`|PlayMontage` (`self.Mesh`) "/Game/Characters/Souls/combat/HitReact_Montage.HitReact_Montage"
    (:`then`
      (set `CharacterMovementComponent.MaxWalkSpeed` 0.0 (`self.CharacterMovement`)))
    (:`OnCompleted`
      (set `CharacterMovementComponent.MaxWalkSpeed` (`self.Initial Walk Speed`) (`self.CharacterMovement`) :!label _label))
    (:`OnInterrupted`
      (goto _label))))

(event `/Game/BluePrints/BP_DAMAGE.End SwordTrace_`
  ;[0.01458 0.01458 0.01458] Sword Traces
  (if (`KismetSystemLibrary.K2_IsValidTimerHandle` (stale `/Game/BluePrints/BP_DAMAGE.Begin SwordTrace` _returnvalue))
    (`KismetSystemLibrary.K2_ClearAndInvalidateTimerHandle` (stale `/Game/BluePrints/BP_DAMAGE.Begin SwordTrace` _returnvalue))))

(event `/Game/BluePrints/BP_DAMAGE.Begin SwordTrace`
  ;[0.01458 0.01458 0.01458] Sword Traces
  (bind _returnvalue (`KismetSystemLibrary.K2_SetTimerDelegate` (delegate `damage trace`) 0.01 true)))

(event `damage trace`
  ;[0.01458 0.01458 0.01458] Sword Traces
  (if (not (`self.isDead?`))
    (bind (_outhit _returnvalue) (`KismetSystemLibrary.SphereTraceSingleForObjects` :`Start` (`KismetMathLibrary.SelectVector` (`self.Start Sword Trace Boss`) (`SceneComponent.K2_GetComponentLocation` (`self.Start Sword Trace Pos`)) (`self.ISBoss`)) :`End` (`KismetMathLibrary.SelectVector` (`self.End Sword Trace Boss`) (`SceneComponent.K2_GetComponentLocation` (`self.End Sword Trace Pos`)) (`self.ISBoss`)) :`Radius` (`self.SwordTraceRadius`) :`ObjectTypes` (`|MakeArray` "ObjectTypeQuery3" :!type "EObjectTypeQuery Enum") :`DrawDebugType` "ForOneFrame" :`DrawTime` 0.5))
    (if _returnvalue
      (`/Engine/EditorBlueprintResources/StandardMacros.DoOnce` false :!label _label_2
        (:`Completed`
          (`GameplayStatics.ApplyDamage` (`.HitActor` (`GameplayStatics.BreakHitResult` _outhit)) (`self.SwordDamage`))
          (`KismetSystemLibrary.Delay` 0.3)
          (goto _label_2 :!via `Reset`))))))

(event `/Game/BluePrints/BP_DAMAGE.die`
  ;[0.01458 0.01458 0.01458] BOSS AI
  (`CharacterMovementComponent.DisableMovement` (`self.CharacterMovement`))
  (`PrimitiveComponent.SetSimulatePhysics` (`self.Mesh`) true)
  (set `self.isDead?` true))

(event `/Game/BluePrints/BP_DAMAGE.Point Damage Trace`
  (bind _returnvalue (`SceneComponent.K2_GetComponentLocation` (`self.PointTrace Pos`)))
  (bind _returnvalue_2 (`SceneComponent.K2_GetComponentLocation` (`self.PointTrace Pos`)))
  ;[0.01458 0.01458 0.01458] BOSS AI
  (`|ExecutionSequence`
    (:`then_0`
      (bind (_outhit _returnvalue_3) (`KismetSystemLibrary.SphereTraceSingleForObjects` :`Start` _returnvalue_2 :`End` _returnvalue_2 :`Radius` (`self.AttackRadius`) :`ObjectTypes` (`|MakeArray` "ObjectTypeQuery3" :!type "EObjectTypeQuery Enum") :`DrawDebugType` "ForDuration"))
      (if _returnvalue_3
        (`GameplayStatics.ApplyDamage` (`.HitActor` (`GameplayStatics.BreakHitResult` _outhit)) 10.0)))
    (:`then_1`
      (`GameplayStatics.PlaySoundAtLocation` "/Game/Audio/Sounds/MS_BigAttack.MS_BigAttack" _returnvalue (struct) 1.0 1.0 0.0 null null null null)
      (`GameplayStatics.PlayWorldCameraShake` "/Game/BluePrints/BP_CAMERA_SHAKE_ATTACK.BP_CAMERA_SHAKE_ATTACK_C" _returnvalue 0.0 2000.0)
      (`GameplayStatics.SpawnEmitterAtLocation` null _returnvalue (struct) (1.0 1.0 1.0) true "AutoRelease"))))

(event `self.Trigger.OnComponentBeginOverlap`
  (params (OverlappedComponent :type "PrimitiveComponent Object Reference") (OtherActor :type "Actor Object Reference") (OtherComp :type "PrimitiveComponent Object Reference") (OtherBodyIndex :type Integer) (bFromSweep :type Boolean) (SweepResult :type "HitResult Structure (by ref)"))
  (if (`KismetSystemLibrary.DoesImplementInterface` OtherActor "/Game/BluePrints/Weapons/BPI_Interact.BPI_Interact_C")
    (`SceneComponent.SetVisibility` (`self.Widget`) true false)))

(event `self.Trigger.OnComponentEndOverlap`
  (params (OverlappedComponent :type "PrimitiveComponent Object Reference") (OtherActor :type "Actor Object Reference") (OtherComp :type "PrimitiveComponent Object Reference") (OtherBodyIndex :type Integer))
  (if (`KismetSystemLibrary.DoesImplementInterface` OtherActor "/Game/BluePrints/Weapons/BPI_Interact.BPI_Interact_C")
    (`SceneComponent.SetVisibility` (`self.Widget`) false false)))

(fn `Big Attack`
  (returns (Duration :type "Float (double-precision)"))
  (bind _returnvalue (`self.PlayAnimMontage` (`self.BigAttackMontage`)))
  (`GameplayStatics.PlaySoundAtLocation` "/Game/Audio/Sounds/C_GruxAttack.C_GruxAttack" (`self.K2_GetActorLocation`) (struct) 1.0 1.0 0.0 null null null null)
  (return _returnvalue))

(fn `Sword Attack`
  (returns (Duration :type "Float (double-precision)"))
  (bind _returnvalue (`self.PlayAnimMontage` (`self.SwordAttack Montage`)))
  (`GameplayStatics.PlaySoundAtLocation` (`self.SwordAttck Sound`) (`self.K2_GetActorLocation`) (struct) 1.0 1.0 0.0 null null null null)
  (return _returnvalue))

(fn `UserConstructionScript`)