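; BPC_Stats is a component that tracks its owner's health and stamina and keeps their progress bars in sync.
; IncreaseValue adjusts the chosen stat, clamps it between zero and its maximum, and updates the matching bar if valid.
; A fast looping timer started at BeginPlay refills stamina while the RegainStamina flag is set.
; When a health change leaves it at zero, Die sends DieMessage to the owning actor.
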(event `self.ReceiveBeginPlay`
  (`KismetSystemLibrary.K2_SetTimerDelegate` (delegate `Regain Stamina`) 0.01 true))

(event `Regain Stamina`
  (if (`self.RegainStamina`)
    (`self.increase value` "NewEnumerator1" 0.1)))

(event `die`
  (message `/Game/BluePrints/BP_DAMAGE.die` (`self.GetOwner`)))

(event `Set Health Progress BAR`
  (params (`healthProgress bar ` :type "ProgressBar Object Reference"))
  (set `self.Health Progress Bar` `healthProgress bar `))

(event `SetStaminaProgressbar`
  (params (`Stamina Progress Bar` :type "ProgressBar Object Reference"))
  (set `self.Stamina Progress Bar` `Stamina Progress Bar`))

(fn `increase value`
  (params (stats :type "/Game/BluePrints/E_stats Enum" :default "NewEnumerator0") (value :type "Float (double-precision)"))
  (switch `/Game/BluePrints/E_stats` stats
    (:`NewEnumerator0`
      (set `self.health` (`KismetMathLibrary.FClamp` (+ (`self.health`) value) 0.0 (`self.Maxheath`)))
      (`|ExecutionSequence`
        (:`then_0`
          (if (<= (`self.health`) 0.0)
            (`self.die`)))
        (:`then_1`
          (bind _health_progress_bar (`self.Health Progress Bar`)
            (:`then`
              (`ProgressBar.SetPercent` _health_progress_bar (/ (`self.health`) (`self.Maxheath`))))
            (:`else`)))))
    (:`NewEnumerator1`
      (set `self.Stamina` (`KismetMathLibrary.FClamp` (+ (`self.Stamina`) value) 0.0 (`self.MaxStamina`)))
      (bind _stamina_progress_bar (`self.Stamina Progress Bar`)
        (:`then`
          (`ProgressBar.SetPercent` _stamina_progress_bar (/ (`self.Stamina`) (`self.MaxStamina`))))
        (:`else`)))))