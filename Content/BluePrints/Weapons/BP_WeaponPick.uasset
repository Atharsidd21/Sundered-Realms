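; BP_WeaponPick is a world weapon pickup that hands its WeaponData to whatever overlaps it.
; The construction script sets the visible static mesh from WeaponData, so one Blueprint serves any weapon.
; On trigger overlap, actors implementing BPI_Interact receive a PickupWeaponMessage with the data, then the pickup plays an attenuated equip sound at its location and destroys itself.
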(event `self.Pickup Trigger.OnComponentBeginOverlap`
  (params (OverlappedComponent :type "PrimitiveComponent Object Reference") (OtherActor :type "Actor Object Reference") (OtherComp :type "PrimitiveComponent Object Reference") (OtherBodyIndex :type Integer) (bFromSweep :type Boolean) (SweepResult :type "HitResult Structure (by ref)"))
  (if (`KismetSystemLibrary.DoesImplementInterface` OtherActor "/Game/BluePrints/Weapons/BPI_Interact.BPI_Interact_C")
    (message `/Game/BluePrints/Weapons/BPI_Interact.Pickup Weapon` OtherActor (`self.Weapon Data`))
    (`GameplayStatics.PlaySoundAtLocation` "/Game/Audio/Sounds/item-equip-6904.item-equip-6904" (`self.K2_GetActorLocation`) (struct) 1.0 1.0 0.0 "/Game/Audio/Sounds/SA_Character.SA_Character" null null null)
    (`self.K2_DestroyActor`)))

(fn `UserConstructionScript`
  (`StaticMeshComponent.SetStaticMesh` (`self.StaticMesh`) (`/Game/BluePrints/Weapons/BP_DA_Weapon.Static Mesh` (`self.Weapon Data`))))